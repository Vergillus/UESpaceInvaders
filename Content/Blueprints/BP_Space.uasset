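; BP_Space is an actor with a Plane whose material can follow the horizontal screen position of a Player actor.
; BeginPlay creates a dynamic material instance for the Plane, then switches actor tick off.
; When ticking, it projects the Player's location to screen, divides X by viewport width and writes the result to a scalar material parameter.
; Nothing in this Blueprint re-enables tick or assigns Player.
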(event EventBeginPlay
  (bind _plane (Variables|Default|GetPlane))
  (bind _returnvalue (Rendering|Material|CreateDynamicMaterialInstance (Rendering|Material|GetMaterial _plane 0) "None" "None" :!class /Script/Engine.KismetMaterialLibrary))
  (bind _output_get (Variables|Default|SetDynamicMat _returnvalue))
  (Rendering|Material|SetMaterial _plane 0 _output_get)
  (Actor|Tick|SetActorTickEnabled false))

(event Collision|EventActorBeginOverlap
  (params (OtherActor :type Actor%20Object%20Reference)))

(event EventTick
  (params (DeltaSeconds :type Float%20%28single-precision%29))
  (bind _returnvalue (Game|GetPlayerController 0))
  (Rendering|Material|SetScalarParameterValue (Variables|Default|GetDynamicMat) "Param" (/ (.x (.ScreenPosition (Class|GameplayStatics|ProjectWorldtoScreen _returnvalue (Transformation|GetActorLocation (Variables|Default|GetPlayer)) false))) (.SizeX (HUD|GetViewportSize _returnvalue))) :!class /Script/Engine.MaterialInstanceDynamic))

(fn ConstructionScript)